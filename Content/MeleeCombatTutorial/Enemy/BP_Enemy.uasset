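; Melee enemy that chases the player on sight, turns to face them and swings a sword.
; Pawn sensing triggers AI MoveTo; on arrival, Tick interpolates yaw until aligned, then plays a wind-up and attack montage.
; Animation-toggled hitbox sphere-traces along blade sockets, damaging the Player-tagged actor once per swing.
; Damage interrupts attacks with a hit reaction, ignores further hits until it ends, and destroys the enemy at zero health.
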(event OnSeePawn(PawnSensing)
  (params (Pawn :type Pawn%20Object%20Reference))
  (Variables|AttackValues|SetIsSeeingPlayer true)
  (CallFunction|FollowPlayer))

(event Custom|FollowPlayer
  (if (Math|Boolean|ANDBoolean (Variables|AttackValues|GetIsSeeingPlayer) (not (Variables|AttackValues|GetIsAttacking)) (not (Variables|AttackValues|GetIsTryingToFacePlayer)))
    (AI|AIMoveTo self "0, 0, 0" (Game|GetPlayerCharacter 0) 2e+02 false
      (:OnSuccess
        (if (not (Variables|AttackValues|GetIsTryingToFacePlayer))
          (Variables|AttackValues|SetIsTryingToFacePlayer true)))
      (:OnFail
        (if (Variables|AttackValues|GetIsTryingToFacePlayer)
          (Variables|AttackValues|SetIsTryingToFacePlayer false))))))

(event Custom|EnableSwordHitbox
  ;[0.05098 0.05098 0.05098] Events for enabling and disabling the hitbox through animation
  (Variables|AttackValues|SetHitboxEnabled true))

(event Custom|DisableSwordHitbox
  ;[0.05098 0.05098 0.05098] Events for enabling and disabling the hitbox through animation
  (Variables|AttackValues|SetHitboxEnabled false))

(event Custom|CheckHitbox
  (bind _mesh (Variables|Character|GetMesh))
  ;[0.05098 0.05098 0.05098] Attack Logic - Checks if the hitbox is enabled and if so, checks the sword's path for any enemies
  (if (Variables|AttackValues|GetHitboxEnabled)
    (bind _outhits (Collision|MultiSphereTraceForObjects (Transformation|GetSocketLocation _mesh "socket_blade_start") (Transformation|GetSocketLocation _mesh "socket_blade_end") (Variables|AttackValues|GetAttackHitboxRadius) (Utilities|Array|MakeArray "ObjectTypeQuery3") false 0 "ForDuration" true "(R=1.000000,G=0.000000,B=0.000000,A=1.000000)" "(R=0.000000,G=1.000000,B=0.000000,A=1.000000)" 1.0))
    (for _array_element _outhits
      (if (and (Actor|ActorHasTag (.HitActor (Collision|BreakHitResult _array_element)) "Player") (not (Variables|AttackValues|GetPlayerHit)))
        (Game|Damage|ApplyDamage (.HitActor (Collision|BreakHitResult _array_element)) 1.0 0 0)
        (Variables|AttackValues|SetPlayerHit true)))))

(event Custom|TryFacePlayer
  (if (Variables|AttackValues|GetIsTryingToFacePlayer)
    (bind _iswithinrange (CallFunction|FacePlayer 15.0 1e+01))
    (if _iswithinrange
      (Variables|AttackValues|SetIsAttacking true)
      (Variables|AttackValues|SetIsTryingToFacePlayer false)
      (CallFunction|Attack))))

(event Custom|Attack
  (Animation|PlayAnimMontage "/Game/MeleeCombatTutorial/Enemy/Melee_Attack_Blend_Montage.Melee_Attack_Blend_Montage" 0.0 "None")
  (Utilities|FlowControl|Delay 0.4)
  (if (Variables|AttackValues|GetIsAttacking)
    (bind _returnvalue (Animation|PlayAnimMontage "/Game/MeleeCombatTutorial/Enemy/Melee_Attack_02_A_Montage.Melee_Attack_02_A_Montage" 1.0 "None"))
    (Utilities|FlowControl|Delay (- _returnvalue 0.4))
    (Variables|AttackValues|SetIsAttacking false)
    (Variables|AttackValues|SetPlayerHit false)))

(event EventBeginPlay
  (Variables|AttackValues|SetHealth 3.0))

(event EventTick
  (params (DeltaSeconds :type Float%20%28single-precision%29))
  (Utilities|FlowControl|Sequence
    (:then_0
      (CallFunction|TryFacePlayer))
    (:then_1
      (CallFunction|CheckHitbox))))

(event Game|Damage|EventAnyDamage
  (params (Damage :type Float%20%28single-precision%29) (DamageType :type Damage%20Type%20Object%20Reference) (InstigatedBy :type Controller%20Object%20Reference) (DamageCauser :type Actor%20Object%20Reference))
  (Utilities|FlowControl|DoOnce false :!label _label
    (:Completed
      (bind _output_get (Variables|AttackValues|SetHealth (- (Variables|AttackValues|GetHealth) Damage)))
      (if (<= _output_get 0.0)
        (Actor|DestroyActor)
        (else
          (Variables|AttackValues|SetIsAttacking false)
          (Animation|StopAnimMontage 0)
          (bind _returnvalue (Animation|PlayAnimMontage "/Game/MeleeCombatTutorial/Enemy/Melee_Hit_Front_05_A_Montage.Melee_Hit_Front_05_A_Montage" 1.0 "None"))
          (Utilities|FlowControl|Delay _returnvalue)
          (goto _label Reset))))))

(fn ConstructionScript)

(fn FacePlayer
  (params (InterpolationSpeed :type Float%20%28double-precision%29) (AcceptableRotationRange :type Float%20%28double-precision%29))
  (Transformation|SetActorRotation (Math|Rotator|MakeRotator 0.0 0.0 (.yaw (Math|Interpolation|RInterpTo (Transformation|GetActorRotation) (Math|Rotator|FindLookatRotation (Transformation|GetActorLocation) (Transformation|GetActorLocation (Game|GetPlayerCharacter 0))) (Utilities|Time|GetWorldDeltaSeconds) InterpolationSpeed))))
  (return (<= (Math|Float|Absolute(Float) (- (.yaw (Transformation|GetActorRotation)) (.yaw (Math|Rotator|FindLookatRotation (Transformation|GetActorLocation) (Transformation|GetActorLocation (Game|GetPlayerCharacter 0)))))) AcceptableRotationRange)))